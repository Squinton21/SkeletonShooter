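; Cell door Blueprint that swings open when the player presses the Action input nearby with a high enough score.
; A Box overlap enables input on the door and end overlap disables it.
; On Action, it compares the FirstPersonCharacter's Score against the sum of KeysRequired, EnemiesDefeated and TargetsDestroyed.
; If met, the OpenCloseDoor timeline plays forward to drive the mesh's relative yaw, with no reverse path.
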(event OnComponentBeginOverlap(Box)
  (params (OverlappedComponent :type Primitive%20Component%20Object%20Reference) (OtherActor :type Actor%20Object%20Reference) (OtherComp :type Primitive%20Component%20Object%20Reference) (OtherBodyIndex :type Integer) (bFromSweep :type Boolean) (SweepResult :type Hit%20Result%20Structure%20%28by%20ref%29))
  (Input|EnableInput (Game|GetPlayerController 0)))

(event OnComponentEndOverlap(Box)
  (params (OverlappedComponent :type Primitive%20Component%20Object%20Reference) (OtherActor :type Actor%20Object%20Reference) (OtherComp :type Primitive%20Component%20Object%20Reference) (OtherBodyIndex :type Integer))
  (Input|DisableInput (Game|GetPlayerController 0)))

(event EventBeginPlay)

(event Collision|EventActorBeginOverlap
  (params (OtherActor :type Actor%20Object%20Reference)))

(event Input|ActionEvents|InputActionAction
  (params (Key :type Key%20Structure :default "None"))
  (:Pressed
    (bind _asfirst_person_character (Utilities|Casting|CastToFirstPersonCharacter (Game|GetPlayerCharacter 0)))
    (if (>= (Variables|/Game/FirstPersonBP/Blueprints/FirstPersonCharacter.FirstPersonCharacter_C|GetScore _asfirst_person_character) (+ (Variables|Default|GetKeys%20Required) (Variables|Default|GetEnemies%20Defeated) (Variables|Default|GetTargets%20Destroyed)))
      (bind _newtrack_0 (Timeline|Open/Close%20Door Play)
        (:Update
          (Transformation|SetRelativeRotation (Variables|Debug|GetStaticMeshComponent) (Math|Rotator|MakeRotator 0.0 0.0 _newtrack_0) false false))))))

(fn ConstructionScript)