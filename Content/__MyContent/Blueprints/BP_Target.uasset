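; Shootable target actor that scores and disappears when a first-person projectile enters its Box component.
; The overlap adds one to Score1, stored directly on the HUD widget reached through the game manager, then destroys the actor and plays a 2D sound.
; It also increments the TotalTargets count on player 0's FirstPersonCharacter.
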(event OnComponentBeginOverlap(Box)
  (params (OverlappedComponent :type Primitive%20Component%20Object%20Reference) (OtherActor :type Actor%20Object%20Reference) (OtherComp :type Primitive%20Component%20Object%20Reference) (OtherBodyIndex :type Integer) (bFromSweep :type Boolean) (SweepResult :type Hit%20Result%20Structure%20%28by%20ref%29))
  (Utilities|Casting|CastToFirstPersonProjectile OtherActor)
  (bind _my_game_manager (CallFunction|GetMyGameManager))
  (Variables|/Game/__MyContent/UI/Widget_HUD.Widget_HUD_C|SetScore1 (Variables|/Game/__MyContent/Blueprints/BP_MyGameManager.BP_MyGameManager_C|GetWidget%20HUD _my_game_manager) (+ (Variables|/Game/__MyContent/UI/Widget_HUD.Widget_HUD_C|GetScore1 (Variables|/Game/__MyContent/Blueprints/BP_MyGameManager.BP_MyGameManager_C|GetWidget%20HUD _my_game_manager)) 1))
  (Actor|DestroyActor)
  (Audio|PlaySound2D "/Game/__MyContent/Sounds/Target.Target" 1.0 1.0 0.0 0 0)
  (bind _asfirst_person_character (Utilities|Casting|CastToFirstPersonCharacter (Game|GetPlayerCharacter 0)))
  (Variables|/Game/FirstPersonBP/Blueprints/FirstPersonCharacter.FirstPersonCharacter_C|SetTotal%20Targets _asfirst_person_character (+ (Variables|/Game/FirstPersonBP/Blueprints/FirstPersonCharacter.FirstPersonCharacter_C|GetTotal%20Targets _asfirst_person_character) 1.0)))

(event EventBeginPlay)

(event Collision|EventActorBeginOverlap
  (params (OtherActor :type Actor%20Object%20Reference)))

(event EventTick
  (params (DeltaSeconds :type Float%20%28single-precision%29)))

(fn ConstructionScript)