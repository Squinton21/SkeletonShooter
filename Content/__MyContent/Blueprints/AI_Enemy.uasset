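; Skeleton enemy AI that chases the player, deals contact damage and has a health bar widget.
; PawnSensing triggers a chase sound, sprint animation and SimpleMoveToActor toward the seen pawn.
; Entering the Box applies one capped hit to the tagged player; ContinueDamage is never called here.
; SetHealth caps health, updates the widget and, at zero, destroys the enemy, plays a death sound and increments the player's kill count.
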(event OnSeePawn(PawnSensing)
  (params (Pawn :type Pawn%20Object%20Reference))
  ;[1 1 1] Enemy Follow
  (Audio|PlaySound2D "/Game/__MyContent/Sounds/SkeletonChase.SkeletonChase" 1.0 1.0 0.0 0 0)
  (Components|Animation|PlayAnimation (Variables|Default|GetSkeletalMesh) "/Game/__MyContent/Blueprints/Animation/Charger_Alert_Sprint.Charger_Alert_Sprint" false)
  (AI|Navigation|SimpleMovetoActor (Pawn|GetController) Pawn))

(event OnComponentBeginOverlap(Box)
  (params (OverlappedComponent :type Primitive%20Component%20Object%20Reference) (OtherActor :type Actor%20Object%20Reference) (OtherComp :type Primitive%20Component%20Object%20Reference) (OtherBodyIndex :type Integer) (bFromSweep :type Boolean) (SweepResult :type Hit%20Result%20Structure%20%28by%20ref%29))
  (if (Actor|ActorHasTag OtherActor "My Player")
    (bind _asfirst_person_character (Utilities|Casting|CastToFirstPersonCharacter OtherActor))
    (Variables|Default|SetInside%20Volume true)
    (Variables|Default|SetMy%20Player _asfirst_person_character)
    (CallFunction|StartDamage)))

(event OnComponentEndOverlap(Box)
  (params (OverlappedComponent :type Primitive%20Component%20Object%20Reference) (OtherActor :type Actor%20Object%20Reference) (OtherComp :type Primitive%20Component%20Object%20Reference) (OtherBodyIndex :type Integer))
  (if (Actor|ActorHasTag OtherActor "My Player")
    (Utilities|Casting|CastToFirstPersonCharacter OtherActor)
    (Variables|Default|SetInside%20Volume false)))

(event EventBeginPlay
  (bind _asenemy_health (Utilities|Casting|CastToEnemy_Health (UserInterface|GetUserWidgetObject (Variables|Default|GetEnemy_Health))))
  (Variables|Default|SetEnemy%20Health _asenemy_health)
  (CallFunction|Init))

(fn ConstructionScript)

(fn StartDamage
  (bind _output_get (Variables|Default|SetAccum%20Damage (Variables|Default|GetInstant%20Damage)))
  (if (> _output_get (Variables|Default|GetMax%20Damage))
    (Variables|Default|SetAccum%20Damage (Variables|Default|GetMax%20Damage)))
  (Default|ChangeHealth (Variables|Default|GetMy%20Player) (* (Variables|Default|GetAccum%20Damage) -1.0)))

(fn ContinueDamage
  (bind _returnvalue (Utilities|Time|GetWorldDeltaSeconds))
  (bind _damage_rate (Variables|Default|GetDamage%20Rate))
  (bind _returnvalue_2 (* _damage_rate _returnvalue))
  (if (< (Variables|Default|GetAccum%20Damage) (Variables|Default|GetMax%20Damage))
    (Variables|Default|SetAccum%20Damage (+ _returnvalue_2 (Variables|Default|GetAccum%20Damage)))
    (CallFunction|ChangeHealth (* _returnvalue_2 0.0))))

(fn SetHealth
  (params (Health%20Points :type Float%20%28single-precision%29))
  (bind _output_get (Variables|Default|SetEnemyHealth Health%20Points))
  (if (> _output_get 1e+01)
    (Variables|Default|SetEnemyHealth 1e+01))
  (if (<= _output_get 0.0)
    (Variables|Default|SetEnemyHealth 0.0)
    (Actor|DestroyActor)
    (Audio|PlaySound2D "/Game/__MyContent/Sounds/SkeletonDeath.SkeletonDeath" 1.0 1.0 0.0 0 0)
    (bind _asfirst_person_character (Utilities|Casting|CastToFirstPersonCharacter (Game|GetPlayerCharacter 0)))
    (Variables|/Game/FirstPersonBP/Blueprints/FirstPersonCharacter.FirstPersonCharacter_C|SetEnemies%20Killed _asfirst_person_character (+ (Variables|/Game/FirstPersonBP/Blueprints/FirstPersonCharacter.FirstPersonCharacter_C|GetEnemies%20Killed _asfirst_person_character) 1.0))
    (else
      (Variables|/Game/__MyContent/UI/Enemy_Health.Enemy_Health_C|SetEnemyHealth (Variables|Default|GetEnemy%20Health) (/ (Variables|Default|GetEnemyHealth) 1e+01)))))

(fn GetHealth
  (return (Variables|Default|GetEnemyHealth)))

(fn Init
  (CallFunction|SetHealth 2e+01))

(fn ChangeHealth
  (params (Delta%20Points :type Float%20%28single-precision%29))
  (CallFunction|SetHealth (+ Delta%20Points (Variables|Default|GetEnemyHealth))))