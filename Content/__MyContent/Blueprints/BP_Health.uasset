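; BP_Health is a health pickup that restores a fixed amount of health to the first-person player character.
; Its static mesh spins continuously on Tick.
; When the character overlaps its box, it adds health, writes the normalized value to the HUD widget via the game manager, plays a sound and destroys itself.
; The added health is not clamped to a maximum.
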(event OnComponentBeginOverlap(Box)
  (params (OverlappedComponent :type Primitive%20Component%20Object%20Reference) (OtherActor :type Actor%20Object%20Reference) (OtherComp :type Primitive%20Component%20Object%20Reference) (OtherBodyIndex :type Integer) (bFromSweep :type Boolean) (SweepResult :type Hit%20Result%20Structure%20%28by%20ref%29))
  (bind _asfirst_person_character (Utilities|Casting|CastToFirstPersonCharacter OtherActor))
  (bind _output_get (Variables|/Game/FirstPersonBP/Blueprints/FirstPersonCharacter.FirstPersonCharacter_C|SetHealth%20Points _asfirst_person_character (+ (Variables|/Game/FirstPersonBP/Blueprints/FirstPersonCharacter.FirstPersonCharacter_C|GetHealth%20Points _asfirst_person_character) 25.0)))
  (bind _my_game_manager (CallFunction|GetMyGameManager))
  (Variables|/Game/__MyContent/UI/Widget_HUD.Widget_HUD_C|SetHealth1 (Variables|/Game/__MyContent/Blueprints/BP_MyGameManager.BP_MyGameManager_C|GetWidget%20HUD _my_game_manager) (/ _output_get 1e+02))
  (Actor|DestroyActor)
  (Audio|PlaySound2D "/Game/__MyContent/Sounds/Health.Health" 1.0 1.0 0.0 0 0))

(event EventBeginPlay)

(event Collision|EventActorBeginOverlap
  (params (OtherActor :type Actor%20Object%20Reference)))

(event EventTick
  (params (DeltaSeconds :type Float%20%28single-precision%29))
  (Transformation|AddRelativeRotation (Variables|Default|GetStaticMesh) (Math|Rotator|MakeRotator 0.0 0.0 (* DeltaSeconds 9e+01)) false false))

(fn ConstructionScript)